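; Game instance Blueprint that hosts and joins multiplayer sessions through Advanced Sessions nodes.
; OpenLevel sets up a session, then on success opens the play world level as a listen server and issues a voice loopback console command.
; FindLevel searches all server types and joins the first result on success, with no check for an empty list.
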(event `OpenLevel`
  (`CreateSessionCallbackProxyAdvanced.CreateAdvancedSession` :`PlayerController` (`GameplayStatics.GetPlayerController` 0)
    (:`OnSuccess`
      (bind _returnvalue (`self.GetPlayWorldLevel`))
      (`GameplayStatics.OpenLevel` (`KismetStringLibrary.Conv_StringToName` _returnvalue) true "Listen")
      (`KismetSystemLibrary.ExecuteConsoleCommand` "OSS.VoiceLoopback1" null))))

(event `FindLevel`
  (bind _returnvalue (`GameplayStatics.GetPlayerController` 0))
  (bind _results (`FindSessionsCallbackProxyAdvanced.FindSessionsAdvanced` _returnvalue 10 false "AllServers")
    (:`OnSuccess`
      (`JoinSessionCallbackProxy.JoinSession` _returnvalue (`|GetArrayItem` _results)))))