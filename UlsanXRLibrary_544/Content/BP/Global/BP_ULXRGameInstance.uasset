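; BP_ULXRGameInstance is a game instance Blueprint that hosts and joins LAN multiplayer sessions through Advanced Sessions nodes.
; OpenLevel creates a LAN session with 50 public connections, then opens the level returned by GetPlayWorldLevel as a listen server.
; FindLevel searches the LAN for a single session and joins the first result, printing a message on success.
; Neither event handles failure, and the join does not check that a result exists.
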(event `OpenLevel`
  (`CreateSessionCallbackProxyAdvanced.CreateAdvancedSession` :`PlayerController` (`GameplayStatics.GetPlayerController` 0) :`PublicConnections` 50 :`bUseLAN` true :`bUseLobbiesVoiceChatIfAvailable` true
    (:`OnSuccess`
      (bind _returnvalue (`self.GetPlayWorldLevel`))
      (`GameplayStatics.OpenLevel` (`KismetStringLibrary.Conv_StringToName` _returnvalue) true "Listen"))))

(event `FindLevel`
  (bind _returnvalue (`GameplayStatics.GetPlayerController` 0))
  (bind _results (`FindSessionsCallbackProxyAdvanced.FindSessionsAdvanced` _returnvalue 1 true "AllServers")
    (:`OnSuccess`
      (`JoinSessionCallbackProxy.JoinSession` _returnvalue (`|GetArrayItem` _results)
        (:`OnSuccess`
          (`KismetSystemLibrary.PrintString` "Join Sucesses"))))))