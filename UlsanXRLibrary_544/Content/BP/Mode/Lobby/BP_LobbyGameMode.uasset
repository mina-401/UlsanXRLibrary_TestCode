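; Lobby game mode that initializes voice chat on player characters whenever a player joins.
; PostLogin and HandleStartingNewPlayer run duplicate logic, polling with a short Retriggerable Delay until the new player controls a BP_PlayCharacter.
; They then loop through the GameState PlayerArray and call InitVOIPComp on every player's character, not just the newcomer's.
; Missing pawns trigger the same delayed retry from inside the loop.
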(event `self.K2_PostLogin`
  (params (NewPlayer :type "PlayerController Object Reference"))
  (cast `/Game/BP/Mode/Play/BP_PlayCharacter` (`Controller.K2_GetPawn` NewPlayer) :!label _label
    (:`then`
      (for _array_element (`GameStateBase.PlayerArray` (`GameplayStatics.GetGameState`))
        (bind _returnvalue (`Controller.K2_GetPawn` (`PlayerState.GetPlayerController` _array_element)))
        (`/Engine/EditorBlueprintResources/StandardMacros.IsValid` _returnvalue :!label _label_2
          (:`Is Valid`
            (bind _asbp_play_character (cast `/Game/BP/Mode/Play/BP_PlayCharacter` _returnvalue))
            (`/Game/BP/Mode/Play/BP_PlayCharacter.InitVOIPComp` _asbp_play_character))
          (:`Is Not Valid`
            (`KismetSystemLibrary.RetriggerableDelay` 0.2)
            (goto _label_2)))))
    (:`CastFailed`
      (`KismetSystemLibrary.RetriggerableDelay` 0.2)
      (goto _label))))

(event `self.HandleStartingNewPlayer`
  (params (NewPlayer :type "PlayerController Object Reference"))
  (`parent.HandleStartingNewPlayer` NewPlayer)
  (cast `/Game/BP/Mode/Play/BP_PlayCharacter` (`Controller.K2_GetPawn` NewPlayer) :!label _label_3
    (:`then`
      (for _array_element (`GameStateBase.PlayerArray` (`GameplayStatics.GetGameState`))
        (bind _returnvalue (`Controller.K2_GetPawn` (`PlayerState.GetPlayerController` _array_element)))
        (`/Engine/EditorBlueprintResources/StandardMacros.IsValid` _returnvalue :!label _label_4
          (:`Is Valid`
            (bind _asbp_play_character (cast `/Game/BP/Mode/Play/BP_PlayCharacter` _returnvalue))
            (`/Game/BP/Mode/Play/BP_PlayCharacter.InitVOIPComp` _asbp_play_character))
          (:`Is Not Valid`
            (`KismetSystemLibrary.RetriggerableDelay` 0.2)
            (goto _label_4)))))
    (:`CastFailed`
      (`KismetSystemLibrary.RetriggerableDelay` 0.2)
      (goto _label_3))))

(fn `UserConstructionScript`)