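; Playable character for play mode that adds push-to-talk voice chat and helpers for the main play UI.
; InitVOIPComp retries until PlayerState is valid, registers the VOIPTalker with it, then applies mic settings through console commands for the local player.
; The IA_Voice input starts and stops networked voice.
; Other events turn a server-travel book actor toward the camera above the character, and fetch or toggle WBP_PlayMain widgets.
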(event `VoiceSetting`
  (bind _returnvalue (`GameplayStatics.GetPlayerController` 0))
  ;[0.15 0.15 0.15 0.5 106] 음성 세팅
  (if (`self.IsLocallyControlled`)
    (`KismetSystemLibrary.ExecuteConsoleCommand` "voice.MicInputGain 5" _returnvalue)
    (`KismetSystemLibrary.ExecuteConsoleCommand` "voice.MicNoiseGateThreshold -1" _returnvalue)))

(event `EnhancedInput|/Game/ThirdPerson/Input/Actions/IA_Move`
  (params (ActionValue :type "Vector2D Structure") (ElapsedSeconds :type "Float (double-precision)") (TriggeredSeconds :type "Float (double-precision)") (InputAction :type "InputAction Object Reference" :default "/Game/ThirdPerson/Input/Actions/IA_Move.IA_Move")))

(event `ClearVoicePackets`)

(event `InitVOIPComp`
  (bind _playerstate (`self.PlayerState`))
  ;[0.15 0.15 0.15 0.5 74] VOIP 붙이기
  (`/Engine/EditorBlueprintResources/StandardMacros.IsValid` _playerstate :!label _label
    (:`Is Valid`
      (`VOIPTalker.RegisterWithPlayerState` (`self.VOIPTalker`) _playerstate)
      (`VOIPStatics.SetMicThreshold` -2.0)
      (set `VOIPTalker.Settings` (make `VoiceSettings` (`self.CapsuleComponent`)) (`self.VOIPTalker`))
      (`self.VoiceSetting`))
    (:`Is Not Valid`
      (`KismetSystemLibrary.Delay` 0.2)
      (goto _label))))

(event `Client_CloseVoice`)

(event `EnhancedInput|/Game/BP/Mode/Play/Input/IA_Voice`
  (params (ActionValue :type Boolean) (ElapsedSeconds :type "Float (double-precision)") (TriggeredSeconds :type "Float (double-precision)") (InputAction :type "InputAction Object Reference" :default "/Game/BP/Mode/Play/Input/IA_Voice.IA_Voice"))
  (:`Started`
    (`self.VOIPTalker`
      (:`then`
        (`AdvancedVoiceLibrary.StartNetworkedVoice` 0))
      (:`else`)))
  (:`Completed`
    (`AdvancedVoiceLibrary.StopNetworkedVoice` 0)))

(event `self.ActorLookAtCamera`
  (params (_Actor :type "Actor Object Reference"))
  (bind (_returnvalue_roll _returnvalue_pitch _returnvalue_yaw) (`KismetMathLibrary.BreakRotator` (`KismetMathLibrary.Conv_VectorToRotator` (`KismetMathLibrary.Normal` (- (`SceneComponent.K2_GetComponentLocation` (`self.CameraComponent`)) (`self.K2_GetActorLocation`))))))
  ;[0 0.01609 0.15 0.5 50] 서버 이동용 Book , 항상 카메라 방향으로 회전하기
  (`self.K2_SetActorRotation` _Actor (`KismetMathLibrary.MakeRotator` _returnvalue_roll 0.0 _returnvalue_yaw) false)
  (`self.K2_SetActorLocation` _Actor (+ (`self.K2_GetActorLocation`) (0.0 0.0 200.0)) false false))

(event `self.GetWidgetFromMain`
  (params (_Type :type "ETitleUIType Enum" :default "TitleRoom"))
  ;[0.15 0.15 0.15 0.5 66] 위젯 가져오기
  (bind _foundwidgets (`WidgetBlueprintLibrary.GetAllWidgetsOfClass` "/Game/BP/Mode/Play/UI/WBP_PlayMain.WBP_PlayMain_C"))
  (bind _returnvalue (`TitleUserWidget.GetWidget` (`|GetArrayItem` _foundwidgets) _Type))
  (set `self.CurWidget` _returnvalue))

(event `self.VisibleChangeUIFromAllWidget`
  (params (_Type :type "ETitleUIType Enum" :default "TitleRoom") (_Value :type "ESlateVisibility Enum" :default "Visible"))
  ;[0.15 0.15 0.15 0.5 66] 위젯 가져오기
  (bind _foundwidgets (`WidgetBlueprintLibrary.GetAllWidgetsOfClass` "/Game/BP/Mode/Play/UI/WBP_PlayMain.WBP_PlayMain_C"))
  (`TitleUserWidget.VisibleChangeUI` (`|GetArrayItem` _foundwidgets) _Type _Value))

(fn `UserConstructionScript`)